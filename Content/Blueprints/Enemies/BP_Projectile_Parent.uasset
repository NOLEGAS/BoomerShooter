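; Parent projectile Blueprint for enemies that flies forward and damages what it hits.
; Tick moves it along its forward vector at Speed, scaled by delta time, using a swept SetActorLocation rather than a movement component.
; On overlap with any actor other than its Instigator, it sends HurtMessage with Damage, prints the hit actor's name and destroys itself.
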(event `self.ReceiveTick`
  (params (DeltaSeconds :type "Float (single-precision)"))
  ; Moves projectile
  (set `self.Delta Seconds` DeltaSeconds)
  (`self.K2_SetActorLocation` self (+ (* (`self.GetActorForwardVector` self) (`self.speed`) (`self.Delta Seconds`)) (`self.K2_GetActorLocation` self)) true false))

(event `self.ReceiveActorBeginOverlap`
  (params (OtherActor :type "Actor Object Reference"))
  ; Damages whatever is hit and destroys projectile
  (if (!= OtherActor (`self.GetInstigator`))
    (message `/Game/Blueprints/BPI_Damage.Hurt` OtherActor (`self.damage`))
    (`KismetSystemLibrary.PrintString` (`KismetSystemLibrary.GetDisplayName` OtherActor))
    (`self.K2_DestroyActor`)))

(fn `UserConstructionScript`)