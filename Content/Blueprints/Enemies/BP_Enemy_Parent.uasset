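; BP_Enemy_Parent is an enemy base Blueprint that handles health, death and a temporary overhead health bar.
; Hurt and Heal adjust health, push current and max values to the WBP_EnemyHealth widget, then show it for a set duration through a shared Delay.
; Max health is captured from starting health on BeginPlay, Heal does not clamp to it, and death destroys the actor.
; A helper function sets the movement component's walk speed.
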(event `self.ReceiveBeginPlay`
  (set `self.maxEnemyHealth` (`self.enemyHealth`)))

(event `/Game/Blueprints/BPI_Damage.Hurt`
  (params (amount :type "Float (double-precision)"))
  (bind _healthbar (`self.HealthBar`))
  (bind _output_get (set `self.enemyHealth` (- (`self.enemyHealth`) amount)))
  (if (<= _output_get 0.0)
    (`/Game/Blueprints/BPI_Damage.Death`)
    (else
      ; Briefly shows the health bar
      (`self.UpdateHealthbar`)
      (`SceneComponent.SetVisibility` _healthbar true false :!label _label)
      (`KismetSystemLibrary.Delay` (`self.healthBarShowDuration`))
      (`SceneComponent.SetVisibility` _healthbar false false))))

(event `/Game/Blueprints/BPI_Damage.Heal`
  (params (amount :type "Float (double-precision)"))
  (set `self.enemyHealth` (+ (`self.enemyHealth`) amount))
  (`self.UpdateHealthbar`)
  (goto _label))

(event `/Game/Blueprints/BPI_Damage.Death`
  (`self.K2_DestroyActor`))

(fn `UpdateHealthbar`
  (bind _aswbp_enemy_health (cast `/Game/UI/WBP_EnemyHealth` (`WidgetComponent.GetUserWidgetObject` (`self.HealthBar`))))
  (set `/Game/UI/WBP_EnemyHealth.health` (`self.enemyHealth`) _aswbp_enemy_health)
  (set `/Game/UI/WBP_EnemyHealth.maxHealth` (`self.maxEnemyHealth`) _aswbp_enemy_health)
  (return))

(fn `UpdateWalkSpeed`
  (params (newWalkSpeed :type "Float (double-precision)"))
  (set `CharacterMovementComponent.MaxWalkSpeed` newWalkSpeed (`self.CharacterMovement`)))

(fn `UserConstructionScript`)