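; AI controller for the Shooter enemy that runs the BT_Shooter behavior tree on possession.
; A perception update that senses a Player-tagged actor cancels the forget timer and writes that actor and line of sight to the Blackboard.
; Any other update, including one for a non-player actor, starts a LineOfSightTimer delay that then clears both keys.
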(event `self.ReceivePossess`
  (params (PossessedPawn :type "Pawn Object Reference"))
  (`self.RunBehaviorTree` "/Game/Blueprints/Enemies/BT_Shooter.BT_Shooter"))

(event `self.AIPerception.OnTargetPerceptionUpdated`
  (params (Actor :type "Actor Object Reference") (Stimulus :type "AIStimulus Structure"))
  (bind _blackboard (`self.Blackboard`))
  (if (and (`self.ActorHasTag` Actor "Player") (`.bSuccessfullySensed` (break `AIStimulus` Stimulus)))
    (`KismetSystemLibrary.K2_ClearAndInvalidateTimerHandle` (`self.enemyTimer`))
    (`BlackboardComponent.SetValueAsBool` _blackboard (`self.hasLineOfSight`) true)
    (`BlackboardComponent.SetValueAsObject` _blackboard (`self.enemyActor`) Actor)
    (else
      (bind _returnvalue (`KismetSystemLibrary.K2_SetTimerDelegate` (delegate `StartEnemyTimer`) (`self.lineOfSightTimer`)))
      (set `self.enemyTimer` _returnvalue))))

(event `StartEnemyTimer`
  (bind _blackboard (`self.Blackboard`))
  (`BlackboardComponent.SetValueAsBool` _blackboard (`self.hasLineOfSight`) false)
  (`BlackboardComponent.SetValueAsObject` _blackboard (`self.enemyActor`) null))

(fn `UserConstructionScript`)