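; BP_HealthPack is a pickup that heals the player on touch and then removes itself.
; When its capsule is overlapped, it checks that the actor is a BP_FirstPersonCharacter, is the first player's pawn, and is not at max health.
; A DoOnce then guards a single HealMessage call carrying HealAmount, after which the pack is destroyed.
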(event `self.Capsule.OnComponentBeginOverlap`
  (params (OverlappedComponent :type "PrimitiveComponent Object Reference") (OtherActor :type "Actor Object Reference") (OtherComp :type "PrimitiveComponent Object Reference") (OtherBodyIndex :type Integer) (bFromSweep :type Boolean) (SweepResult :type "HitResult Structure (by ref)"))
  (bind _asbp_first_person_character (cast `/Game/FirstPerson/Blueprints/BP_FirstPersonCharacter` OtherActor))
  (if (== OtherActor (`GameplayStatics.GetPlayerPawn` 0))
    (if (not (== (`/Game/FirstPerson/Blueprints/BP_FirstPersonCharacter.playerHealth` _asbp_first_person_character) (`/Game/FirstPerson/Blueprints/BP_FirstPersonCharacter.maxPlayerHealth` _asbp_first_person_character)))
      (`/Engine/EditorBlueprintResources/StandardMacros.DoOnce` false
        (:`Completed`
          (message `/Game/Blueprints/BPI_Damage.Heal` OtherActor (`self.healAmount`))
          (`self.K2_DestroyActor`))))))

(fn `UserConstructionScript`)